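; PlayerCamera is a camera actor that makes itself the first player's view and follows the player pawn along the world X axis.
; Every Tick it calls SetViewTargetWithBlend on itself with no BeginPlay setup.
; When the pawn is valid, it moves to a fixed offset behind the pawn's X position, keeping its own Y and Z unchanged.
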(event `self.ReceiveTick`
  (params (DeltaSeconds :type "Float (single-precision)"))
  (bind _returnvalue (`GameplayStatics.GetPlayerPawn` 0))
  (`PlayerController.SetViewTargetWithBlend` (`GameplayStatics.GetPlayerController` 0) self 0.0 "VTBlend_Linear" 0.0 false)
  (`/Engine/EditorBlueprintResources/StandardMacros.IsValid` _returnvalue
    (:`Is Valid`
      (`self.K2_SetActorLocation` (`KismetMathLibrary.MakeVector` (+ (.x (`self.K2_GetActorLocation` _returnvalue)) -330.0) (.y (`self.K2_GetActorLocation`)) (.z (`self.K2_GetActorLocation`)))))))

(fn `UserConstructionScript`)