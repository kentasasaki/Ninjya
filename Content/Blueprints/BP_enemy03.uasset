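; BP_enemy03 is an enemy actor that advances along negative Y once the player pawn is near on that axis.
; Tick steps its location a fixed amount each frame, not scaled by delta time, prints the new Y, and destroys the actor once it falls far enough behind the player.
; Overlap of Box_0 with an actor tagged Player sets an AttackOn flag, which nothing in these graphs reads.
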(event `self.ReceiveTick`
  (params (DeltaSeconds :type "Float (single-precision)"))
  (if (<= (- (.y (`self.K2_GetActorLocation`)) (.y (`self.K2_GetActorLocation` (`GameplayStatics.GetPlayerPawn` 0)))) 1000.0)
    (bind _output_get (set `self.move` (- (.y (`self.K2_GetActorLocation`)) 10.0)))
    (`KismetSystemLibrary.PrintString` (`KismetStringLibrary.Conv_DoubleToString` _output_get))
    (`self.K2_SetActorLocation` (`KismetMathLibrary.MakeVector` (.x (`self.K2_GetActorLocation`)) _output_get (.z (`self.K2_GetActorLocation`))))
    (if (<= (.y (`self.K2_GetActorLocation`)) (- (.y (`self.K2_GetActorLocation` (`GameplayStatics.GetPlayerPawn` 0))) 400.0))
      (`self.K2_DestroyActor`))))

(event `self.Box_0.OnComponentBeginOverlap`
  (params (OverlappedComponent :type "PrimitiveComponent Object Reference") (OtherActor :type "Actor Object Reference") (OtherComp :type "PrimitiveComponent Object Reference") (OtherBodyIndex :type Integer) (bFromSweep :type Boolean) (SweepResult :type "HitResult Structure (by ref)"))
  ;[1 1 1] 攻撃
  (if (`self.ActorHasTag` OtherActor "Player")
    (set `self.Attack_on` true)))

(fn `UserConstructionScript`
  (`parent.UserConstructionScript`))