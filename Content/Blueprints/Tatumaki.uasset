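; Tatumaki (tornado) is a moving hazard actor that damages the player on contact.
; Tick plays a timeline whose updates set the Cube's relative yaw from the actor yaw plus the track value.
; Each update also shifts the actor a fixed step along world -Y without sweep, so speed depends on frame rate.
; When the Cube overlaps a Player-tagged actor, it applies damage and destroys itself.
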(event `self.ReceiveTick`
  (params (DeltaSeconds :type "Float (single-precision)"))
  (bind (_direction `_新規track_0`) (`Timeline|タイムライン_0`)
    (:`Update`
      (`SceneComponent.K2_SetRelativeRotation` (`self.Cube`) (`KismetMathLibrary.MakeRotator` 0.0 0.0 (+ (.yaw (`self.K2_GetActorRotation`)) `_新規track_0`)) false false)
      (bind _output_get (set `self.NewVar_1` (- (.y (`self.K2_GetActorLocation`)) 5.0)))
      (`self.K2_SetActorLocation` (`KismetMathLibrary.MakeVector` (.x (`self.K2_GetActorLocation`)) _output_get (.z (`self.K2_GetActorLocation`)))))))

(event `self.Cube.OnComponentBeginOverlap`
  (params (OverlappedComponent :type "PrimitiveComponent Object Reference") (OtherActor :type "Actor Object Reference") (OtherComp :type "PrimitiveComponent Object Reference") (OtherBodyIndex :type Integer) (bFromSweep :type Boolean) (SweepResult :type "HitResult Structure (by ref)"))
  (if (`self.ActorHasTag` OtherActor "Player")
    (`GameplayStatics.ApplyDamage` OtherActor 1.0)
    (`self.K2_DestroyActor`)))

(fn `UserConstructionScript`)