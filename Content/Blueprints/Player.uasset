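; Player actor for an auto-forward game with clamped sideways movement, gear levels, life and a forward attack.
; Tick advances X and line-traces ahead for "Enemy"-tagged actors, which AttackOn damages.
; W shifts up and resets speed points; S and incoming damage share one path that costs life and downshifts.
; F/R adjust speed points through a timeline-animated gear widget, but the full-points auto-upshift is disconnected.
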(event `moveRight`
  ;[1 1 1] 左右移動
  (if (>= (`self.YPosition`) (`self.value`))
    (set `self.YPosition` (`self.value`))
    (else
      (set `self.YPosition` (+ (`self.YPosition`) (`self.value`)))))
  (`self.K2_SetActorLocation` (`KismetMathLibrary.MakeVector` (.x (`self.K2_GetActorLocation`)) (`self.YPosition`) (.z (`self.K2_GetActorLocation`))) :!label _label))

(event `moveLeft`
  (bind _returnvalue (* (`self.value`) -1.0))
  ;[1 1 1] 左右移動
  (if (<= (`self.YPosition`) _returnvalue)
    (set `self.YPosition` _returnvalue)
    (goto _label)
    (else
      (set `self.YPosition` (- (`self.YPosition`) (`self.value`)))
      (goto _label))))

(event `self.ReceiveTick`
  (params (DeltaSeconds :type "Float (single-precision)"))
  (bind _returnvalue (`self.K2_GetActorLocation`))
  ;[1 1 1] 移動＆攻撃範囲のチェック
  (`self.K2_SetActorLocation` (`KismetMathLibrary.MakeVector` (+ (.x (`self.K2_GetActorLocation`)) (`self.move`)) (.y (`self.K2_GetActorLocation`)) (.z (`self.K2_GetActorLocation`))))
  (bind _outhit (`KismetSystemLibrary.LineTraceSingle` :`Start` _returnvalue :`End` (+ _returnvalue (* (`KismetMathLibrary.GetForwardVector` (`self.K2_GetActorRotation`)) 200.0)) :`TraceChannel` "TraceTypeQuery1" :`DrawDebugType` "ForOneFrame"))
  (bind (_bblockinghit _binitialoverlap _time _distance _location _impactpoint _normal _impactnormal _physmat _hitactor) (`GameplayStatics.BreakHitResult` _outhit))
  (if _bblockinghit
    (if (`self.ActorHasTag` _hitactor "Enemy")
      (set `self.enemy_in` true))
    (else
      (set `self.enemy_in` false))))

(event `Key|W`
  (params (Key :type "Key Structure"))
  (bind (_gia _speed) (break `/Game/Blueprints/Sp` (`self.gia`)))
  ;[1 1 1] 速度UP
  (:`Pressed`
    (if (not (`|EnumEquality` _gia "NewEnumerator4"))
      (bind _output_get (set `self.gia` (make `/Game/Blueprints/Sp` (cast `/Game/Blueprints/Gia` (+ _gia 1)) _speed)))
      (`/Game/Blueprints/Plater_Gia.nunber_UpDown` (`self.gia_widget`) (`KismetMathLibrary.Conv_ByteToInt` (`.Gia_6_BA4E3C98479AE8F8D1FE5F882C14A3B0` (break `/Game/Blueprints/Sp` _output_get))))
      (bind _output_get_2 (set `self.Speedpoint` -1))
      (`/Game/Blueprints/Plater_Gia.gia_upDown` (`self.gia_widget`) _output_get_2))))

(event `Key|S`
  (params (Key :type "Key Structure"))
  (bind (_gia _speed) (break `/Game/Blueprints/Sp` (`self.gia`)))
  ;[1 1 1] 減速
  (:`Pressed`
    (bind _output_get (set `self.Life` (- (`self.Life`) 1) :!label _label_2))
    (`/Game/Blueprints/Player_Life.damage` (`self.life_widget`) _output_get)
    (if (not (`|EnumEquality` _gia "NewEnumerator0"))
      (bind _output_get_2 (set `self.gia` (make `/Game/Blueprints/Sp` (cast `/Game/Blueprints/Gia` (- _gia 1)) _speed)))
      (`/Game/Blueprints/Plater_Gia.nunber_UpDown` (`self.gia_widget`) (`KismetMathLibrary.Conv_ByteToInt` (`.Gia_6_BA4E3C98479AE8F8D1FE5F882C14A3B0` (break `/Game/Blueprints/Sp` _output_get_2)))))))

(event `self.ReceiveAnyDamage`
  (params (Damage :type "Float (single-precision)") (DamageType :type "DamageType Object Reference") (InstigatedBy :type "Controller Object Reference") (DamageCauser :type "Actor Object Reference"))
  ;[1 1 1] 減速
  (goto _label_2))

(event `AttackOn`
  ;[1 1 1] 攻撃
  (set `self.attack` true)
  (if (`self.enemy_in`)
    (`GameplayStatics.ApplyDamage` (`.HitActor` (`GameplayStatics.BreakHitResult` (stale `self.ReceiveTick` _outhit))) 1.0)))

(event `self.ReceiveBeginPlay`
  ;[1 1 1] widgetの設定
  (bind _returnvalue (`|CreateWidget` "/Game/Blueprints/Player_Life.Player_Life_C"))
  (set `self.life_widget` _returnvalue)
  (bind _returnvalue_2 (`|CreateWidget` "/Game/Blueprints/Plater_Gia.Plater_Gia_C"))
  (set `self.gia_widget` _returnvalue_2)
  (`UserWidget.AddToViewport` (`self.life_widget`) 0)
  (`UserWidget.AddToViewport` (`self.gia_widget`) 0))

(event `Key|F`
  (params (Key :type "Key Structure"))
  (bind _speedpoint (`self.Speedpoint`))
  ;[1 1 1] gia_pointUp
  (:`Pressed`
    (if (< _speedpoint 4) :!label _label_3
      (set `self.Speedpoint` (+ _speedpoint 1))
      (bind (_direction `_新規track_1`) (`Timeline|タイムライン_0` :!via `PlayFromStart` :!label _label_4)
        (:`Update`
          (`/Game/Blueprints/Plater_Gia.bladeUP` (`self.gia_widget`) (`self.Speedpoint`) `_新規track_1`)
          (`/Game/Blueprints/Plater_Gia.gia_upDown` (`self.gia_widget`) (`self.Speedpoint`))))
      (else
        (set `self.Speedpoint` 4)))))

(event `SpeedPointUp`
  ;[1 1 1] gia_pointUp
  (goto _label_3))

(event `Key|R`
  (params (Key :type "Key Structure"))
  (bind _speedpoint (`self.Speedpoint`))
  ;[1 1 1] gia_pointDown
  (:`Pressed`
    (if (> _speedpoint -1) :!label _label_5
      (set `self.Speedpoint` (- _speedpoint 1))
      (goto _label_4 :!via `ReverseFromEnd`)
      (else
        (set `self.Speedpoint` -1)))))

(event `SpeedPointDown`
  ;[1 1 1] gia_pointDown
  (goto _label_5))

(fn `UserConstructionScript`)