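; Camera actor that becomes the first player controller's view target on BeginPlay.
; Each Tick it reads the Move value from the Player pawn and adds it to its own Y location, leaving X and Z unchanged.
; The offset is applied per frame without delta-time scaling or sweep, so the camera tracks the value rather than the pawn's position.
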(event `self.ReceiveBeginPlay`
  (`PlayerController.SetViewTargetWithBlend` (`GameplayStatics.GetPlayerController` 0) self 0.0 "VTBlend_Linear" 0.0 false))

(event `self.ReceiveTick`
  (params (DeltaSeconds :type "Float (single-precision)"))
  (`self.K2_SetActorLocation` (`KismetMathLibrary.MakeVector` (.x (`self.K2_GetActorLocation`)) (+ (.y (`self.K2_GetActorLocation`)) (`/Game/Blueprints/Player.move` (cast `/Game/Blueprints/Player` (`GameplayStatics.GetPlayerPawn` 0) :!pure true))) (.z (`self.K2_GetActorLocation`)))))

(fn `UserConstructionScript`)