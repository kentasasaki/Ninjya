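; BP_enemy02 is an enemy that fires a single Tatumaki attack when the player comes within range.
; Each Tick compares its Y position to the player's as a signed difference against a fixed threshold, so only that axis matters.
; A DoOnce gate then raises AttackOn, waits briefly, spawns Tatumaki at the enemy's location and clears the flag.
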(event `self.ReceiveTick`
  (params (DeltaSeconds :type "Float (single-precision)"))
  (bind _returnvalue (`self.K2_GetActorLocation`))
  (if (<= (- (.y _returnvalue) (.y (`self.K2_GetActorLocation` (cast `/Game/Blueprints/Player` (`GameplayStatics.GetPlayerPawn` 0) :!pure true)))) 1500.0)
    (`/Engine/EditorBlueprintResources/StandardMacros.DoOnce` false
      (:`Completed`
        (set `self.Attack_on` true)
        (`KismetSystemLibrary.Delay` 0.5)
        (`|SpawnActorFromClass` "/Game/Blueprints/Tatumaki.Tatumaki_C" (`KismetMathLibrary.MakeTransform` _returnvalue (struct) (1.0 1.0 1.0)) "Undefined" "OverrideRootScale")
        (set `self.Attack_on` false)))))

(fn `UserConstructionScript`
  (`parent.UserConstructionScript`))